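; Hero Blueprint that fires a hitscan shot with cosmetic impact effects on the F key or Fire input.
; A short visibility trace from the camera attaches blood particles and sound to any ThirdPersonCharacter hit; other hits and misses spawn an explosion at the hit result's location.
; Blood particle collisions spawn short-lived, randomly sized splatter decals aligned to the surface, using dynamic materials with a random frame.
; No damage is applied.
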(event Custom|ColisionarSuelo
  (params (EventName :type Name) (EmitterTime :type Float%20%28single-precision%29) (ParticleTime :type Integer) (Location :type Vector) (Velocity :type Vector) (Direction :type Vector) (Normal :type Vector) (BoneName :type Name) (PhysMat :type Physical%20Material%20Object%20Reference))
  (bind _returnvalue (Rendering|Material|CreateDynamicMaterialInstance "/Game/M_SplatterTexture.M_SplatterTexture" "None" "None" :!class /Script/Engine.KismetMaterialLibrary))
  (Rendering|Material|SetScalarParameterValue _returnvalue "Frame" (Math|Conversions|ToFloat(Integer) (Math|Random|RandomInteger 11)) :!class /Script/Engine.MaterialInstanceDynamic)
  (Rendering|Decal|SpawnDecalatLocation _returnvalue (Math|Conversions|ToVector(Float) (Math|Random|RandomFloatinRange 2e+01 5e+01)) Location (Math|Conversions|RotationFromXVector Normal) 5.0))

(event Input|ActionEvents|InputActionFire
  (params (Key :type Key%20Structure :default "None"))
  (bind _returnvalue (Game|GetPlayerCameraManager 0))
  (bind _returnvalue_2 (Transformation|GetActorLocation _returnvalue))
  (:Pressed
    (Audio|SpawnSound2D "/Game/StarterContent/Audio/Explosion02.Explosion02" 0.75 1.0 0.0 0)
    (bind (_outhit _returnvalue_3) (Collision|LineTraceByChannel _returnvalue_2 (+ _returnvalue_2 (* (Transformation|GetActorForwardVector _returnvalue) 1e+03)) "TraceTypeQuery1" false (Utilities|Array|MakeArray self) "ForDuration"))
    (if _returnvalue_3
      (Development|PrintString (Utilities|GetDisplayName (.HitActor (Collision|BreakHitResult _outhit))))
      (Utilities|FlowControl|Sequence
        (:then_0
          (bind _asthird_person_character (Utilities|Casting|CastToThirdPersonCharacter (.HitActor (Collision|BreakHitResult _outhit)))
            (:then
              (Audio|SpawnSoundAttached "/Game/SFX_GorePack/wav/stereo_bonus/HSg_blood_impact_l_02_stereo.HSg_blood_impact_l_02_stereo" (Variables|/Script/Engine.Character|GetMesh _asthird_person_character) "None" "0, 0, 0" "0, 0, 0" "KeepRelativeOffset" false 1.0 1.0 0.0 0 0)
              (bind _returnvalue_4 (Effects|SpawnEmitterAttached "/Game/P_Blood.P_Blood" (Variables|/Script/Engine.Character|GetMesh _asthird_person_character) "None" "0, 0,150.000000"))
              (EventDispatchers|BindEventtoOnParticleCollide _returnvalue_4 (delegate Custom|ColisionarSuelo)))
            (:CastFailed
              (Audio|SpawnSoundatLocation 0 (.Location (Collision|BreakHitResult _outhit)) "0, 0, 0" 1.0 1.0 0.0 0 0 :!label _label)
              (Effects|SpawnEmitteratLocation "/Game/StarterContent/Particles/P_Explosion.P_Explosion" (.Location (Collision|BreakHitResult _outhit)))))))
      (else
        (goto _label)))))

(event Input|KeyboardEvents|F
  (params (Key :type Key%20Structure :default "None"))
  (bind _returnvalue (Game|GetPlayerCameraManager 0))
  (bind _returnvalue_2 (Transformation|GetActorLocation _returnvalue))
  (:Pressed
    (Audio|SpawnSound2D "/Game/StarterContent/Audio/Explosion02.Explosion02" 0.75 1.0 0.0 0)
    (bind (_outhit _returnvalue_3) (Collision|LineTraceByChannel _returnvalue_2 (+ _returnvalue_2 (* (Transformation|GetActorForwardVector _returnvalue) 1e+03)) "TraceTypeQuery1" false (Utilities|Array|MakeArray self) "ForDuration"))
    (if _returnvalue_3
      (Development|PrintString (Utilities|GetDisplayName (.HitActor (Collision|BreakHitResult _outhit))))
      (Utilities|FlowControl|Sequence
        (:then_0
          (bind _asthird_person_character (Utilities|Casting|CastToThirdPersonCharacter (.HitActor (Collision|BreakHitResult _outhit)))
            (:then
              (Audio|SpawnSoundAttached "/Game/SFX_GorePack/wav/stereo_bonus/HSg_blood_impact_l_02_stereo.HSg_blood_impact_l_02_stereo" (Variables|/Script/Engine.Character|GetMesh _asthird_person_character) "None" "0, 0, 0" "0, 0, 0" "KeepRelativeOffset" false 1.0 1.0 0.0 0 0)
              (bind _returnvalue_4 (Effects|SpawnEmitterAttached "/Game/P_Blood.P_Blood" (Variables|/Script/Engine.Character|GetMesh _asthird_person_character) "None" "0, 0,150.000000"))
              (EventDispatchers|BindEventtoOnParticleCollide _returnvalue_4 (delegate Custom|ColisionarSuelo)))
            (:CastFailed
              (Audio|SpawnSoundatLocation 0 (.Location (Collision|BreakHitResult _outhit)) "0, 0, 0" 1.0 1.0 0.0 0 0 :!label _label)
              (Effects|SpawnEmitteratLocation "/Game/StarterContent/Particles/P_Explosion.P_Explosion" (.Location (Collision|BreakHitResult _outhit)))))))
      (else
        (goto _label)))))

(fn ConstructionScript)